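; Player character Blueprint that handles movement relative to the control rotation and a gated jump.
; Each tick, a visibility line trace from the Sphere component along its up vector sets OnGround by whether the hit actor has the "jump" tag, leaving it unchanged when nothing is hit.
; Jump input fires only while OnGround is true.
; Movement axis inputs are scaled down by DivideAxisBy.
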(event `self.ReceiveTick`
  (params (DeltaSeconds :type "Float (single-precision)"))
  (bind _sphere (`self.Sphere`))
  (bind _returnvalue (`SceneComponent.K2_GetComponentLocation` _sphere))
  ;[1 1 1] Check if on ground
  (bind (_outhit _returnvalue_2) (`KismetSystemLibrary.LineTraceSingle` :`Start` _returnvalue :`End` (+ _returnvalue (* (`KismetMathLibrary.GetUpVector` (`SceneComponent.K2_GetComponentRotation` _sphere)) (`self.distance`))) :`TraceChannel` "TraceTypeQuery1" :`DrawDebugType` "ForDuration" :`DrawTime` 1.0))
  (bind (_bblockinghit _binitialoverlap _time _distance _location _impactpoint _normal _impactnormal _physmat _hitactor) (`GameplayStatics.BreakHitResult` _outhit))
  (`/Engine/EditorBlueprintResources/StandardMacros.IsValid` _hitactor
    (:`Is Valid`
      (if _returnvalue_2
        (if (`self.ActorHasTag` _hitactor "jump")
          (set `self.onGround` true)
          (else
            (set `self.onGround` false)))))))

(event `InputAction|Jump`
  (params (Key :type "Key Structure"))
  (:`Pressed`
    (if (`self.onGround`)
      (`self.Jump`))))

(event `InputAxis|Forward-Back`
  (params (AxisValue :type "Float (single-precision)"))
  (`self.AddMovementInput` (`KismetMathLibrary.GetForwardVector` (`self.GetControlRotation`)) (/ AxisValue (`self.divideAxisBy`))))

(event `InputAxis|Right-Left`
  (params (AxisValue :type "Float (single-precision)"))
  (`self.AddMovementInput` (`KismetMathLibrary.GetRightVector` (`self.GetControlRotation`)) (/ AxisValue (`self.divideAxisBy`))))

(fn `UserConstructionScript`)